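; ScanActor displays a RealSense 3D scan as a vertex-colored procedural mesh that the user can rotate for inspection.
; LoadMesh loads a scan file through the Scan3D component, builds a mesh section from its buffers and resets the scene rotation, while HideMesh hides it.
; Keys spin the actor each Tick, and mouse axes rotate the scene component, with middle button switching horizontal motion from yaw to roll.
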(event EventBeginPlay
  (Input|EnableInput (Game|GetPlayerController 0))
  (Development|ExecuteConsoleCommand "stat fps")
  (Variables|/Script/Engine.PlayerController|SetbShowMouseCursor (Game|GetPlayerController 0) true))

(event EventTick
  (params (DeltaSeconds :type Float%20%28single-precision%29))
  ;[1 1 1] Rotate the Actor
  (Transformation|AddActorLocalRotation (Class|KismetMathLibrary|MakeRot (Variables|Default|GetPitch) (Variables|Default|GetYaw) (Variables|Default|GetRoll)) false))

(event Input|AxisEvents|InputAxisMouseX
  (params (AxisValue :type Float%20%28single-precision%29))
  ;[1 1 1] Rotate self around the X or Z axis, dependent on the middle button state
  (if (Variables|Default|GetMiddleButton)
    (Transformation|AddWorldRotation (Variables|Default|GetScene) (Math|Rotator|MakeRotator 0.0 0.0 AxisValue) false)
    (else
      (Transformation|AddWorldRotation (Variables|Default|GetScene) (Math|Rotator|MakeRotator 0.0 AxisValue 0.0) false))))

(event Input|AxisEvents|InputAxisMouseY
  (params (AxisValue :type Float%20%28single-precision%29))
  ;[1 1 1] Rotate self about the Y axis
  (Transformation|AddWorldRotation (Variables|Default|GetScene) (Math|Rotator|MakeRotator AxisValue 0.0 0.0) false))

(event Input|KeyboardEvents|W
  (:Pressed
    (Variables|Default|SetPitch 1.0))
  (:Released
    (Variables|Default|SetPitch 0.0)))

(event Input|KeyboardEvents|A
  (:Pressed
    (Variables|Default|SetRoll -1.0))
  (:Released
    (Variables|Default|SetRoll 0.0)))

(event Input|KeyboardEvents|S
  (:Pressed
    (Variables|Default|SetPitch -1.0))
  (:Released
    (Variables|Default|SetPitch 0.0)))

(event Input|KeyboardEvents|D
  (:Pressed
    (Variables|Default|SetRoll 1.0))
  (:Released
    (Variables|Default|SetRoll 0.0)))

(event Input|KeyboardEvents|Q
  (:Pressed
    (Variables|Default|SetYaw -1.0))
  (:Released
    (Variables|Default|SetYaw 0.0)))

(event Input|KeyboardEvents|E
  (:Pressed
    (Variables|Default|SetYaw 1.0))
  (:Released
    (Variables|Default|SetYaw 0.0)))

(event Input|MouseEvents|MiddleMouseButton
  (:Pressed
    (Variables|Default|SetMiddleButton true))
  (:Released
    (Variables|Default|SetMiddleButton false)))

(fn ConstructionScript)

(fn LoadMesh
  (params (Filename :type String))
  (bind _scan3d (Variables|Default|GetScan3D))
  (bind _proceduralmesh (Variables|Default|GetProceduralMesh))
  ;[1 1 1] Create a Procedural Mesh from the 3D Scan Component's Vertices, Triangles, and Colors buffer
  (Class|Scan3DComponent|LoadScan (Variables|Default|GetScan3D) Filename)
  (Class|ProceduralMeshComponent|CreateMeshSection _proceduralmesh 0 (Variables|/Script/RealSensePlugin.Scan3DComponent|GetVertices _scan3d) (Variables|/Script/RealSensePlugin.Scan3DComponent|GetTriangles _scan3d) 0 0 (Variables|/Script/RealSensePlugin.Scan3DComponent|GetColors _scan3d) 0 false)
  (Rendering|Material|SetMaterial _proceduralmesh 0 "/Game/RealSense/3DScan/Materials/VertexColorMat.VertexColorMat")
  (Rendering|SetVisibility (Variables|Default|GetProceduralMesh) true false)
  (Transformation|SetWorldRotation (Variables|Default|GetScene) "90.000000,0.000000, 0" false))

(fn HideMesh
  (Rendering|SetVisibility (Variables|Default|GetProceduralMesh) false false))