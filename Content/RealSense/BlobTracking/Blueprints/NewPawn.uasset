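; Pawn that moves a sword with RealSense blob tracking, running the camera from BeginPlay to EndPlay.
; The first detected blob anchors control at the sword's current location.
; On later ticks with a blob, frame-to-frame center movement is axis-remapped, negated, filtered for jitter and spikes, then scaled and added to a target position.
; The sword follows that target through interpolated, swept world-location moves.
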(event EventTick
  (params (DeltaSeconds :type Float%20%28single-precision%29))
  (if (> (Variables|/Script/RealSensePlugin.BlobTrackingComponent|GetBlobCount (Variables|Default|GetBlobTracking)) 0)
    (if (Variables|Default|GetBlobControl)
      (CallFunction|CalcPositionDifferential)
      (Variables|Default|SetTargetPosition (+ (Variables|Default|GetTargetPosition) (Variables|Default|GetPositionDifferential)))
      (bind _output_get (Variables|Default|SetCurrentPosition (Math|Interpolation|VInterpTo (Variables|Default|GetCurrentPosition) (Variables|Default|GetTargetPosition) (Utilities|Time|GetWorldDeltaSeconds) (Variables|Default|GetInterpolationSpeed))))
      (Transformation|SetWorldLocation (Variables|Default|GetSword) _output_get true false)
      (Variables|Default|SetBaseBlobPosition (Variables|/Script/RealSensePlugin.BlobTrackingComponent|GetBlobCenter (Variables|Default|GetBlobTracking)))
      (else
        (CallFunction|SetupSwordControl)))))

(event EventEndPlay
  (params (EndPlayReason :type EEndPlayReason%20Enum :default "Destroyed"))
  (Class|RealSenseComponent|StopCamera (Variables|Default|GetBlobTracking)))

(event EventBeginPlay
  (Class|RealSenseComponent|StartCamera (Variables|Default|GetBlobTracking)))

(fn ConstructionScript)

(fn SetupSwordControl
  (Variables|Default|SetBaseBlobPosition (Variables|/Script/RealSensePlugin.BlobTrackingComponent|GetBlobCenter (Variables|Default|GetBlobTracking)))
  (bind _output_get (Variables|Default|SetCurrentPosition (Transformation|GetWorldLocation (Variables|Default|GetSword))))
  (Variables|Default|SetTargetPosition _output_get)
  (Variables|Default|SetBlobControl true)
  (return))

(fn CalcPositionDifferential
  (bind _baseblobposition (Variables|Default|GetBaseBlobPosition))
  (bind _blobtracking (Variables|Default|GetBlobTracking))
  (bind _blobcenter (Variables|/Script/RealSensePlugin.BlobTrackingComponent|GetBlobCenter _blobtracking))
  (bind _returnvalue (- _blobcenter _baseblobposition))
  (LocalVariables|SetX (* (.z _returnvalue) -1.0))
  (LocalVariables|SetY (* (.x _returnvalue) -1.0))
  (LocalVariables|SetZ (* (.y _returnvalue) -1.0))
  (if (or (< (Math|Float|Absolute(Float) (LocalVariables|GetX)) 5.0) (> (Math|Float|Absolute(Float) (LocalVariables|GetX)) 1e+02))
    (LocalVariables|SetX 0.0))
  (if (or (< (Math|Float|Absolute(Float) (LocalVariables|GetY)) 5.0) (> (Math|Float|Absolute(Float) (LocalVariables|GetY)) 1e+02))
    (LocalVariables|SetY 0.0))
  (if (or (< (Math|Float|Absolute(Float) (LocalVariables|GetZ)) 5.0) (> (Math|Float|Absolute(Float) (LocalVariables|GetZ)) 1e+02))
    (LocalVariables|SetZ 0.0))
  (Variables|Default|SetPositionDifferential (* (Math|Vector|MakeVector (LocalVariables|GetX) (LocalVariables|GetY) (LocalVariables|GetZ)) 2.0))
  (return))