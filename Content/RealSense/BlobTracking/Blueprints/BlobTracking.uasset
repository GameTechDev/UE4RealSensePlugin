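; Actor that uses a RealSense blob tracking camera, started on BeginPlay and stopped on EndPlay, to move itself with a tracked blob.
; Movement logic runs on ActorBeginOverlap, not Tick: the first detection stores baseline blob and actor positions.
; Later overlaps remap the blob-center delta axes, discard jitter and large jumps per axis, then scale it into a target position approached with VInterpTo.
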(event EventActorBeginOverlap
  (params (OtherActor :type Actor%20Object%20Reference))
  (if (> (Variables|/Script/RealSensePlugin.BlobTrackingComponent|GetBlobCount (Variables|Default|GetBlobTracking)) 0)
    (if (Variables|Default|GetBlobControl)
      (CallFunction|CalcPositionDifferential)
      (Variables|Default|SetTargetPosition (+ (Variables|Default|GetTargetPosition) (Variables|Default|GetPositionDifferential)))
      (bind _output_get (Variables|Default|SetCurrentPosition (Math|Interpolation|VInterpTo (Variables|Default|GetCurrentPosition) (Variables|Default|GetTargetPosition) (Utilities|Time|GetWorldDeltaSeconds) (Variables|Default|GetInterpolationSpeed))))
      (Transformation|SetActorLocation _output_get false false)
      (Variables|Default|SetBaseBlobPosition (Variables|/Script/RealSensePlugin.BlobTrackingComponent|GetBlobCenter (Variables|Default|GetBlobTracking)))
      (else
        (CallFunction|SetupBlobControl)))))

(event EventTick
  (params (DeltaSeconds :type Float%20%28single-precision%29)))

(event EventEndPlay
  (params (EndPlayReason :type EEndPlayReason%20Enum :default "Destroyed"))
  (Class|RealSenseComponent|StopCamera (Variables|Default|GetBlobTracking)))

(event EventBeginPlay
  (Class|RealSenseComponent|StartCamera (Variables|Default|GetBlobTracking)))

(fn ConstructionScript)

(fn SetupBlobControl
  (Variables|Default|SetBaseBlobPosition (Variables|/Script/RealSensePlugin.BlobTrackingComponent|GetBlobCenter (Variables|Default|GetBlobTracking)))
  (bind _output_get (Variables|Default|SetCurrentPosition (Transformation|GetActorLocation)))
  (Variables|Default|SetTargetPosition _output_get)
  (Variables|Default|SetBlobControl true)
  (return))

(fn CalcPositionDifferential
  (bind _baseblobposition (Variables|Default|GetBaseBlobPosition))
  (bind _blobtracking (Variables|Default|GetBlobTracking))
  (bind _blobcenter (Variables|/Script/RealSensePlugin.BlobTrackingComponent|GetBlobCenter _blobtracking))
  (bind _returnvalue (- _blobcenter _baseblobposition))
  (LocalVariables|SetX (* (.z _returnvalue) -1.0))
  (LocalVariables|SetY (* (.x _returnvalue) -1.0))
  (LocalVariables|SetZ (* (.y _returnvalue) -1.0))
  (if (or (< (Math|Float|Absolute(Float) (LocalVariables|GetX)) 5.0) (> (Math|Float|Absolute(Float) (LocalVariables|GetX)) 1e+02))
    (LocalVariables|SetX 0.0))
  (if (or (< (Math|Float|Absolute(Float) (LocalVariables|GetY)) 5.0) (> (Math|Float|Absolute(Float) (LocalVariables|GetY)) 1e+02))
    (LocalVariables|SetY 0.0))
  (if (or (< (Math|Float|Absolute(Float) (LocalVariables|GetZ)) 5.0) (> (Math|Float|Absolute(Float) (LocalVariables|GetZ)) 1e+02))
    (LocalVariables|SetZ 0.0))
  (Variables|Default|SetPositionDifferential (* (Math|Vector|MakeVector (LocalVariables|GetX) (LocalVariables|GetY) (LocalVariables|GetZ)) 2.0))
  (return))