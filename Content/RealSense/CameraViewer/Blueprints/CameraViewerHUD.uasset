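; HUD for a RealSense camera viewer that shows live color and depth streams side by side.
; On BeginPlay it adds the CameraViewerUI widget, shows the mouse cursor, enables input and turns on FPS stats.
; Each DrawHUD fills textures from the RealSense color and depth buffers and draws them scaled and letterboxed in the left and right screen halves.
; Ctrl+S toggles drawing of the streams, which also requires the camera to be running.
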(event EventBeginPlay
  (bind _returnvalue (Game|GetPlayerController 0))
  (Input|EnableInput _returnvalue)
  (bind _returnvalue_2 (UserInterface|CreateWidget "/Game/RealSense/CameraViewer/Blueprints/CameraViewerUI.CameraViewerUI_C"))
  (UserInterface|Viewport|AddtoViewport _returnvalue_2 0)
  (Development|ExecuteConsoleCommand "stat fps")
  (Variables|/Script/Engine.PlayerController|SetbShowMouseCursor _returnvalue true))

(event EventDrawHUD
  (params (SizeX :type Integer) (SizeY :type Integer))
  (bind _realsense (Variables|Default|GetRealSense))
  (bind _realsense_2 (Variables|Default|GetRealSense))
  (bind _realsense_3 (Variables|Default|GetRealSense))
  (bind _realsense_4 (Variables|Default|GetRealSense))
  (bind _returnvalue (Class|CameraStreamComponent|GetColorCameraResolution _realsense))
  (bind _returnvalue_2 (Class|CameraStreamComponent|GetDepthCameraResolution _realsense_4))
  (Variables|Default|SetScreenWidth SizeX)
  (Variables|Default|SetScreenHeight SizeY)
  (if (and (Class|RealSenseComponent|IsCameraRunning (Variables|Default|GetRealSense)) (Variables|Default|GetStreaming))
    ;[1 1 1] Fill the Color Texture with data from the Color Buffer
    (bind _returnvalue_3 (Class|RealSenseBlueprintLibrary|ColorBuffertoTexture (Variables|/Script/RealSensePlugin.CameraStreamComponent|GetColorBuffer _realsense_3) (Variables|/Script/RealSensePlugin.CameraStreamComponent|GetColorTexture _realsense_3)))
    ;[1 1 1] Draw the Color Texture to the screen
    (Class|HUD|DrawTextureSimple _returnvalue_3 (.X%20Position (CallFunction|GetLetterboxPosition (.width _returnvalue) (.height _returnvalue) (/ (Variables|Default|GetScreenWidth) 2) (Variables|Default|GetScreenHeight) (CallFunction|GetTextureScale (.width _returnvalue) (.height _returnvalue) (Variables|Default|GetScreenWidth) (Variables|Default|GetScreenHeight)))) (.Y%20Position (CallFunction|GetLetterboxPosition (.width _returnvalue) (.height _returnvalue) (/ (Variables|Default|GetScreenWidth) 2) (Variables|Default|GetScreenHeight) (CallFunction|GetTextureScale (.width _returnvalue) (.height _returnvalue) (Variables|Default|GetScreenWidth) (Variables|Default|GetScreenHeight)))) (CallFunction|GetTextureScale (.width _returnvalue) (.height _returnvalue) (Variables|Default|GetScreenWidth) (Variables|Default|GetScreenHeight)) false)
    ;[1 1 1] Fill the Depth Texture with data from the Depth Buffer
    (bind _returnvalue_4 (Class|RealSenseBlueprintLibrary|DepthBuffertoTexture (Variables|/Script/RealSensePlugin.CameraStreamComponent|GetDepthBuffer _realsense_2) (Variables|/Script/RealSensePlugin.CameraStreamComponent|GetDepthTexture _realsense_2)))
    ;[1 1 1] Draw the Depth Texture to the screen
    (Class|HUD|DrawTextureSimple _returnvalue_4 (+ (Math|Conversions|ToFloat(Integer) (/ (Variables|Default|GetScreenWidth) 2)) (.X%20Position (CallFunction|GetLetterboxPosition (.width _returnvalue_2) (.height _returnvalue_2) (/ (Variables|Default|GetScreenWidth) 2) (Variables|Default|GetScreenHeight) (CallFunction|GetTextureScale (.width _returnvalue_2) (.height _returnvalue_2) (Variables|Default|GetScreenWidth) (Variables|Default|GetScreenHeight))))) (.Y%20Position (CallFunction|GetLetterboxPosition (.width _returnvalue_2) (.height _returnvalue_2) (/ (Variables|Default|GetScreenWidth) 2) (Variables|Default|GetScreenHeight) (CallFunction|GetTextureScale (.width _returnvalue_2) (.height _returnvalue_2) (Variables|Default|GetScreenWidth) (Variables|Default|GetScreenHeight)))) (CallFunction|GetTextureScale (.width _returnvalue_2) (.height _returnvalue_2) (Variables|Default|GetScreenWidth) (Variables|Default|GetScreenHeight)) false)))

(event Input|KeyboardEvents|CtrlS
  (params (Key :type Key%20Structure :default "AnyKey"))
  ;[1 1 1] Toggle Camera Streaming on and off
  (:Pressed
    (Variables|Default|SetStreaming (not (Variables|Default|GetStreaming)))))

(fn ConstructionScript)