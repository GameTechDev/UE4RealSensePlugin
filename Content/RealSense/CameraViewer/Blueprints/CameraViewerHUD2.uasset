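; CameraViewerHUD2 is a HUD for the RealSense camera viewer that displays the color image from the UserSegmentation component.
; On BeginPlay it sets the 3D segmentation camera resolution preset and starts the camera.
; Each DrawHUD converts the segmentation color buffer to a texture and draws it with a scale proportional to viewport width, sized as a small overlay.
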(event EventDrawHUD
  (params (SizeX :type Integer) (SizeY :type Integer))
  (bind _usersegmentation (Variables|Default|GetUserSegmentation))
  (bind _returnvalue (Class|RealSenseBlueprintLibrary|ColorBuffertoTexture (Variables|/Script/RealSensePlugin.UserSegmentationComponent|GetColorBuffer _usersegmentation) (Variables|/Script/RealSensePlugin.UserSegmentationComponent|GetColorTexture _usersegmentation)))
  (Class|HUD|DrawTextureSimple _returnvalue 0.0 0.0 (/ (.X (Math|Vector2D|BreakVector2D (Viewport|GetViewportSize))) (* 6.4e+02 5.0)) false))

(event EventBeginPlay
  (bind _usersegmentation (Variables|Default|GetUserSegmentation))
  (Class|UserSegmentationComponent|Set3DSegCameraResolution _usersegmentation "RES5")
  (Class|RealSenseComponent|StartCamera _usersegmentation))

(event EventActorBeginOverlap
  (params (OtherActor :type Actor%20Object%20Reference)))

(event EventTick
  (params (DeltaSeconds :type Float%20%28single-precision%29)))

(fn ConstructionScript)